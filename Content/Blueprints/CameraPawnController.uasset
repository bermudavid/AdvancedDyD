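; Player controller for a tile-based tactics game with building placement, driving a CameraPawn with move, zoom and gated mouse pan (edge scrolling is disconnected).
; Cursor traces place a selector decal on instanced-mesh tiles and pick a possessed Entity and its target, which feed attack tests and AI moves to tile centres.
; For one Rol value BeginPlay also creates the HUD, construction manager and ghost building, which ConstructBuilding uses for previews.
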(event EventBeginPlay
  (bind _returnvalue (Math|Transform|MakeTransform "0,0.000000,0.000000"))
  ;[1 1 1] Begin Play
  (Variables|Default|SetbEnableMouseOverEvents true)
  (if (Utilities|Enum|Equal(Enum) (Variables|Default|GetRol) "NewEnumerator0")
    (Variables|Default|SetbShowMouseCursor true)
    (Utilities|FlowControl|Sequence
      (:then_0
        (Utilities|ReferenceCast :!label _label))
      (:then_1
        (Input|SetInputModeGameandUI self 0 "LockAlways" false)
        (Utilities|CreateHuds)
        (UserInterface|Viewport|AddtoViewport (Variables|References|GetMainHudRef) 0))
      (:then_2
        (bind _returnvalue_2 (Game|SpawnActorfromClass "/Game/Blueprints/Constructions/ConstructionManager_BP.ConstructionManager_BP_C" _returnvalue "AlwaysSpawn" 0 0))
        (Variables|References|SetConstructionManagerRef _returnvalue_2))
      (:then_3
        (bind _returnvalue_3 (Game|SpawnActorfromClass "/Game/Blueprints/Buildings/GhostBuilding_BP.GhostBuilding_BP_C" _returnvalue "AlwaysSpawn" 0 self 0))
        (Variables|References|SetGhostBuildingRef _returnvalue_3)))
    (else
      (Variables|Default|SetbShowMouseCursor true)
      (goto _label))))

(event EventConstructBuilding
  (params (MainBuilding :type Building%20Master%20BP%20Class%20Reference))
  (bind _ghostbuildingref (Variables|References|GetGhostBuildingRef))
  ;[1 1 1] Construct Hud Event
  (bind _returnvalue (Game|SpawnActorfromClass MainBuilding (Math|Transform|MakeTransform "0, 0, 0") "Undefined" 0 self 0))
  (bind _asbuilding_master_bp (Utilities|Casting|CastToBuildingMaster_BPClass MainBuilding))
  (Default|KillGhost _ghostbuildingref)
  (Default|OnSpawn _ghostbuildingref (Variables|/Game/Blueprints/Buildings/BuildingMaster_BP.BuildingMaster_BP_C|GetDisplayMesh _returnvalue) _asbuilding_master_bp (Variables|/Game/Blueprints/Buildings/BuildingMaster_BP.BuildingMaster_BP_C|GetConstructionProxy _returnvalue)))

(event EventTick
  (params (DeltaSeconds :type Float%20%28single-precision%29))
  (bind _self self)
  (bind (_worldlocation _worlddirection) (Game|Player|ConvertMouseLocationToWorldSpace _self))
  (bind _outhit (Collision|LineTraceByChannel _worldlocation (+ _worldlocation (* _worlddirection 1.5e+03)) "TraceTypeQuery2" true 0 "None"))
  (Utilities|IsValid (stale _returnvalue)
    (:Is%20Valid
      (Components|DestroyComponent (stale _returnvalue)))
    (:Is%20Not%20Valid
      _))
  (bind _returnvalue (Rendering|Decal|SpawnDecalatLocation "/Game/Meshes/Grid/M_SelectorDecal.M_SelectorDecal" "50.000000,50.000000,50.000000" (.Location (Math|Transform|BreakTransform (.OutInstanceTransform (Components|InstancedStaticMesh|GetInstanceTransform (Variables|/Game/Blueprints/Grid/GridBP.GridBP_C|GetHierarchicalInstancedStaticMesh (Variables|Default|GetTile)) (.HitItem (Collision|BreakHitResult _outhit)) false)))) "0.000000,0.000000,0.000000" 0.0)))

(event Input|ActionEvents|InputActionPan
  (params (Key :type Key%20Structure :default "AnyKey"))
  (bind _camerapawnref (Variables|References|GetCameraPawnRef))
  (bind _returnvalue (Transformation|GetActorRotation _camerapawnref))
  (bind (_roll _pitch _yaw) (Math|Rotator|BreakRotator _returnvalue))
  ;[0.05432 1 0.2203] Camera Movement
  ;;[1 1 1] Pan y
  (:Pressed
    (Variables|Default|SetDisableCamNav true)
    (Utilities|FlowControl|Gate true) ; enters at Open
  )
  (:Released
    (Variables|Default|SetDisableCamNav false)
    (Utilities|FlowControl|Gate true) ; enters at Close
  ))

(event Input|ActionEvents|InputActionPan
  (params (Key :type Key%20Structure :default "AnyKey"))
  (bind _camerapawnref (Variables|References|GetCameraPawnRef))
  (bind _returnvalue (Transformation|GetActorRotation _camerapawnref))
  (bind (_roll _pitch _yaw) (Math|Rotator|BreakRotator _returnvalue))
  ;[0.05432 1 0.2203] Camera Movement
  ;;[1 1 1] Pan X
  (:Pressed
    (Variables|Default|SetDisableCamNav true)
    (Utilities|FlowControl|Gate true) ; enters at Open
  )
  (:Released
    (Variables|Default|SetDisableCamNav false)
    (Utilities|FlowControl|Gate true) ; enters at Close
  ))

(event Input|ActionEvents|InputActionPanReset
  (params (Key :type Key%20Structure :default "AnyKey"))
  (bind _camerapawnref (Variables|References|GetCameraPawnRef))
  (bind _returnvalue (Transformation|GetActorRotation _camerapawnref))
  (bind (_roll _pitch _yaw) (Math|Rotator|BreakRotator _returnvalue))
  ;[0.05432 1 0.2203] Camera Movement
  ;;[1 1 1] Pan Reset
  (:Pressed
    (Transformation|SetActorRotation _camerapawnref (Math|Rotator|MakeRotator _roll 0.0 _yaw))))

(event Input|ActionEvents|InputActionZoomIn
  (params (Key :type Key%20Structure :default "AnyKey"))
  (bind (_springarm _targetarmlength) (|SpringArm))
  ;[0.05432 1 0.2203] Camera Movement
  ;;[1 1 1] Zoom
  (:Pressed
    (Variables|/Script/Engine.SpringArmComponent|SetTargetArmLength _springarm (Math|Float|Clamp(Float) (- _targetarmlength (Variables|Default|GetZoomSensitivity)) 1e+02 (Variables|Default|GetMaxArmDistance)))))

(event Input|ActionEvents|InputActionZoomOut
  (params (Key :type Key%20Structure :default "AnyKey"))
  (bind (_springarm _targetarmlength) (|SpringArm))
  ;[0.05432 1 0.2203] Camera Movement
  ;;[1 1 1] Zoom
  (:Pressed
    (Variables|/Script/Engine.SpringArmComponent|SetTargetArmLength _springarm (Math|Float|Clamp(Float) (+ _targetarmlength (Variables|Default|GetZoomSensitivity)) 1e+02 (Variables|Default|GetMaxArmDistance)))))

(event Input|AxisEvents|InputAxisMoveRight
  (params (AxisValue :type Float%20%28single-precision%29))
  (bind _movesensitivity (CallFunction|MovementSpeedCalculation))
  (bind _fastmovemultiplier (Variables|Default|GetFastMoveMultiplier))
  (bind _camerapawnref (Variables|References|GetCameraPawnRef))
  (bind _transform (Utilities|MovementY AxisValue _movesensitivity _fastmovemultiplier _camerapawnref))
  (bind (_location _rotation _scale) (Math|Transform|BreakTransform _transform))
  (bind (_x _y) (Math|Vector|BreakVector _location))
  ;[0.05432 1 0.2203] Camera Movement
  ;;[1 1 1] Movement Y
  (Transformation|SetActorTransform (Variables|References|GetCameraPawnRef) (Math|Transform|MakeTransform (Math|Vector|MakeVector _x _y 1e+02) _rotation _scale)))

(event Input|AxisEvents|InputAxisMoveForward
  (params (AxisValue :type Float%20%28single-precision%29))
  ;[0.05432 1 0.2203] Camera Movement
  ;;[1 1 1] Movement X
  (Transformation|SetActorTransform (Variables|References|GetCameraPawnRef) (Utilities|MovementX (CallFunction|MovementSpeedCalculation) (Variables|Default|GetFastMoveMultiplier) AxisValue (Variables|References|GetCameraPawnRef))))

(event Input|MouseEvents|MouseY
  (params (AxisValue :type Float%20%28single-precision%29))
  (bind _camerapawnref (Variables|References|GetCameraPawnRef))
  (bind _returnvalue (Transformation|GetActorRotation _camerapawnref))
  (bind (_roll _pitch _yaw) (Math|Rotator|BreakRotator _returnvalue))
  ;[0.05432 1 0.2203] Camera Movement
  ;;[1 1 1] Pan y
  (Utilities|FlowControl|Gate true
    (:Exit
      (Transformation|SetActorRotation (Variables|References|GetCameraPawnRef) (Math|Rotator|MakeRotator _roll (Math|Float|Clamp(Float) (+ _pitch (* AxisValue (Variables|Default|GetPanSensitivity))) -15.0 45.0) _yaw)))))

(event Input|MouseEvents|MouseX
  (params (AxisValue :type Float%20%28single-precision%29))
  ;[0.05432 1 0.2203] Camera Movement
  ;;[1 1 1] Automatic movement at the borders of the screen
)

(event Input|MouseEvents|MouseY
  (params (AxisValue :type Float%20%28single-precision%29))
  ;[0.05432 1 0.2203] Camera Movement
  ;;[1 1 1] Automatic movement at the borders of the screen
)

(event Input|MouseEvents|MouseX
  (params (AxisValue :type Float%20%28single-precision%29))
  (bind _camerapawnref (Variables|References|GetCameraPawnRef))
  (bind _returnvalue (Transformation|GetActorRotation _camerapawnref))
  (bind (_roll _pitch _yaw) (Math|Rotator|BreakRotator _returnvalue))
  ;[0.05432 1 0.2203] Camera Movement
  ;;[1 1 1] Pan X
  (Utilities|FlowControl|Gate true
    (:Exit
      (Transformation|SetActorRotation (Variables|References|GetCameraPawnRef) (Math|Rotator|MakeRotator _roll _pitch (+ _yaw (* AxisValue (Variables|Default|GetPanSensitivity))))))))

(event Input|KeyboardEvents|LeftShift
  (params (Key :type Key%20Structure :default "AnyKey"))
  ;[0.05432 1 0.2203] Camera Movement
  ;;[1 1 1] fast move
  (:Pressed
    (Variables|Default|SetFastMoveMultiplier 2.0))
  (:Released
    (Variables|Default|SetFastMoveMultiplier 1.0)))

(event Input|KeyboardEvents|LeftCtrl
  (params (Key :type Key%20Structure :default "AnyKey"))
  (:Released
    (Utilities|ResetPossesedPawn)
    (Utilities|ResetTargetPawn)))

(event Input|KeyboardEvents|I
  (params (Key :type Key%20Structure :default "AnyKey"))
  ;[1 1 1] Show debug Info
  (:Pressed
    (Development|PrintString (Utilities|String|Append "Pawn Possesed: " (Utilities|GetDisplayName (Variables|References|GetEntityPossesedReference)) " Target: " (Utilities|GetDisplayName (Variables|References|GetTarget))))
    (if (and (Variables|Default|GetPawnPossesed?) (Variables|Default|GetHasTarget?))
      (Class|Entity|DistancetoTarget (Variables|References|GetEntityPossesedReference) (Variables|References|GetTarget))))
  (:Released
    (Rendering|Debug|FlushPersistentDebugLines)
    (Class|KismetSystemLibrary|FlushDebugStrings)))

(event Input|KeyboardEvents|G
  (params (Key :type Key%20Structure :default "AnyKey"))
  (bind _target (Variables|References|GetTarget))
  (bind _pg (Variables|/Script/AdvancedDyD.Entity|Getpg _target))
  (bind _returnvalue (Math|Conversions|ToFloat(Integer) _pg))
  ;[1 1 1] To Attack Test
  (:Released
    ;;[1 1 1] If pawn possessed and has target
    (if (and (Variables|Default|GetPawnPossesed?) (Variables|Default|GetHasTarget?))
      (bind _returnvalue_2 (Class|Entity|ToAttackTest (Variables|References|GetEntityPossesedReference) _target))
      (if _returnvalue_2
        (Development|PrintString "Le diste wey")
        (else
          (Development|PrintString "dale más duro wey")))
      (bind _astest (Utilities|Casting|CastToTest _target))
      (Utilities|FlowControl|Sequence
        (:then_0
          (Default|UpdateHealth (Variables|/Game/Blueprints/Test.Test_C|GetWidgetBar _astest) _returnvalue))
        (:then_1
          (Default|UpdateHealth (Variables|/Game/Blueprints/Test.Test_C|GetWidgetBar2 _astest) _returnvalue))))))

(event Input|MouseEvents|LeftMouseButton
  (params (Key :type Key%20Structure :default "AnyKey"))
  (bind _self self)
  (bind (_worldlocation _worlddirection) (Game|Player|ConvertMouseLocationToWorldSpace _self))
  ;[1 1 1] Selection
  (:Released
    (bind _outhit (Collision|LineTraceByChannel _worldlocation (+ _worldlocation (* _worlddirection 1.5e+04)) "TraceTypeQuery2" false 0 "None" true "(R=1.000000,G=0.000000,B=0.000000,A=1.000000)" "(R=0.529105,G=0.000000,B=1.000000,A=1.000000)"))
    (if (Variables|Default|GetPawnPossesed?)
      (bind _asentity (Utilities|Casting|CastToEntity (.HitActor (Collision|BreakHitResult _outhit))))
      (bind _astest (Utilities|Casting|CastToTest (Variables|References|GetTarget))
        (:then
          (Development|SetHiddeninGame (Variables|/Game/Blueprints/Test.Test_C|GetSelector _astest) true false))
        (:CastFailed
          _))
      (bind _output_get (Variables|References|SetTarget _asentity))
      (Variables|Default|SetHasTarget? true)
      (bind _astest_2 (Utilities|Casting|CastToTest _output_get))
      (bind _returnvalue (Rendering|Material|CreateDynamicMaterialInstance (Variables|/Game/Blueprints/Test.Test_C|GetSelector _astest_2) 0 "/Game/Blueprints/M_Selector.M_Selector" :!class /Script/Engine.PrimitiveComponent))
      (Rendering|Material|SetVectorParameterValue _returnvalue "Color" "(R=0.538819,G=0.885000,B=0.369656,A=1.000000)" :!class /Script/Engine.MaterialInstanceDynamic)
      (Rendering|Material|SetMaterial (Variables|/Game/Blueprints/Test.Test_C|GetSelector _astest_2) 0 _returnvalue)
      (Development|SetHiddeninGame (Variables|/Game/Blueprints/Test.Test_C|GetSelector _astest_2) false false)
      (else
        (bind _asentity_2 (Utilities|Casting|CastToEntity (.HitActor (Collision|BreakHitResult _outhit))))
        (bind _output_get_2 (Variables|References|SetEntityPossesedReference _asentity_2))
        (bind _astest_3 (Utilities|Casting|CastToTest _output_get_2)
          (:then
            (Development|SetHiddeninGame (Variables|/Game/Blueprints/Test.Test_C|GetSelector _astest_3) false false))
          (:CastFailed
            _))
        (Variables|Default|SetPawnPossesed? true)))))

(event Input|MouseEvents|RightMouseButton
  (params (Key :type Key%20Structure :default "AnyKey"))
  (bind _self self)
  (bind _entitypossesedreference (Variables|References|GetEntityPossesedReference))
  (bind (_worldlocation _worlddirection) (Game|Player|ConvertMouseLocationToWorldSpace _self))
  ;[1 1 1] Move Selected to  Location
  (:Released
    (if (CallFunction|PossesedCanMove?)
      (bind _outhit (Collision|LineTraceByChannel _worldlocation (+ _worldlocation (* _worlddirection 1.5e+03)) "TraceTypeQuery2" true 0 "Persistent"))
      (Utilities|FlowControl|Sequence
        (:then_0
          (Class|Entity|DistancetoTransform (Variables|References|GetEntityPossesedReference) (.OutInstanceTransform (Components|InstancedStaticMesh|GetInstanceTransform (Variables|/Game/Blueprints/Grid/GridBP.GridBP_C|GetHierarchicalInstancedStaticMesh (Variables|Default|GetTile)) (.HitItem (Collision|BreakHitResult _outhit)) false)))
          (AI|AIMoveTo (Variables|References|GetEntityPossesedReference) (Math|Vector|MakeVector (.x (.Location (Math|Transform|BreakTransform (.OutInstanceTransform (Components|InstancedStaticMesh|GetInstanceTransform (Variables|/Game/Blueprints/Grid/GridBP.GridBP_C|GetHierarchicalInstancedStaticMesh (Variables|Default|GetTile)) (.HitItem (Collision|BreakHitResult _outhit)) false))))) (.y (.Location (Math|Transform|BreakTransform (.OutInstanceTransform (Components|InstancedStaticMesh|GetInstanceTransform (Variables|/Game/Blueprints/Grid/GridBP.GridBP_C|GetHierarchicalInstancedStaticMesh (Variables|Default|GetTile)) (.HitItem (Collision|BreakHitResult _outhit)) false))))) (+ (.z (.Location (Math|Transform|BreakTransform (.OutInstanceTransform (Components|InstancedStaticMesh|GetInstanceTransform (Variables|/Game/Blueprints/Grid/GridBP.GridBP_C|GetHierarchicalInstancedStaticMesh (Variables|Default|GetTile)) (.HitItem (Collision|BreakHitResult _outhit)) false))))) 46.0)) 0 0.01 true
            (:OnSuccess
              (Variables|/Script/AdvancedDyD.Entity|SetVelocidad _entitypossesedreference (- (Variables|/Script/AdvancedDyD.Entity|GetVelocidad _entitypossesedreference) 0))
              (Rendering|Debug|FlushPersistentDebugLines)
              (Class|KismetSystemLibrary|FlushDebugStrings)
              (Transformation|SetActorLocation _entitypossesedreference (Math|Vector|MakeVector (.x (.Location (Math|Transform|BreakTransform (.OutInstanceTransform (Components|InstancedStaticMesh|GetInstanceTransform (Variables|/Game/Blueprints/Grid/GridBP.GridBP_C|GetHierarchicalInstancedStaticMesh (Variables|Default|GetTile)) (.HitItem (Collision|BreakHitResult _outhit)) false))))) (.y (.Location (Math|Transform|BreakTransform (.OutInstanceTransform (Components|InstancedStaticMesh|GetInstanceTransform (Variables|/Game/Blueprints/Grid/GridBP.GridBP_C|GetHierarchicalInstancedStaticMesh (Variables|Default|GetTile)) (.HitItem (Collision|BreakHitResult _outhit)) false))))) (+ (.z (.Location (Math|Transform|BreakTransform (.OutInstanceTransform (Components|InstancedStaticMesh|GetInstanceTransform (Variables|/Game/Blueprints/Grid/GridBP.GridBP_C|GetHierarchicalInstancedStaticMesh (Variables|Default|GetTile)) (.HitItem (Collision|BreakHitResult _outhit)) false))))) 46.0)) false false))))))))

(fn ConstructionScript)

(fn MovementSpeedCalculation
  (return (Math|Float|Clamp(Float) (/ (Variables|/Script/Engine.SpringArmComponent|GetTargetArmLength (Variables|/Game/Blueprints/CameraPawn.CameraPawn_C|GetSpringArm (Variables|References|GetCameraPawnRef))) 1e+02) 5.0 2e+01)))

(fn PossesedCanMove?
  (return (not (<= (Variables|/Script/AdvancedDyD.Entity|GetVelocidad (Variables|References|GetEntityPossesedReference)) 0))))

(fn FindinGrid
  (params (Location :type Vector)))

(fn SwitchSelector
  (if (Math|Boolean|Equal(Boolean) (LocalVariables|GetSelector) false)
    (LocalVariables|SetSelector true)
    (else
      (LocalVariables|SetSelector false)))
  (return (LocalVariables|GetSelector)))

(fn ShowNeigbors
  (params (InputPin :type Grid%20BP%20Object%20Reference))
  (bind _e (Variables|/Game/Blueprints/Grid/GridBP.GridBP_C|GetE InputPin))
  (bind _n (Variables|/Game/Blueprints/Grid/GridBP.GridBP_C|GetN InputPin))
  (bind _s (Variables|/Game/Blueprints/Grid/GridBP.GridBP_C|GetS InputPin))
  (bind _w (Variables|/Game/Blueprints/Grid/GridBP.GridBP_C|GetW InputPin))
  (bind _nw (Variables|/Game/Blueprints/Grid/GridBP.GridBP_C|GetNW InputPin))
  (bind _ne (Variables|/Game/Blueprints/Grid/GridBP.GridBP_C|GetNE InputPin))
  (bind _sw (Variables|/Game/Blueprints/Grid/GridBP.GridBP_C|GetSW InputPin))
  (bind _se (Variables|/Game/Blueprints/Grid/GridBP.GridBP_C|GetSE InputPin))
  (Utilities|IsValid _e
    (:Is%20Valid
      (Utilities|ResaltarTile _e)
      (Utilities|IsValid _n
        (:Is%20Valid
          (Utilities|ResaltarTile _n)
          (Utilities|IsValid _s
            (:Is%20Valid
              (Utilities|ResaltarTile _s)
              (Utilities|IsValid _w
                (:Is%20Valid
                  (Utilities|ResaltarTile _w)
                  (Utilities|IsValid _nw
                    (:Is%20Valid
                      (Utilities|ResaltarTile _nw)
                      (Utilities|IsValid _ne
                        (:Is%20Valid
                          (Utilities|ResaltarTile _ne)
                          (Utilities|IsValid _sw
                            (:Is%20Valid
                              (Utilities|ResaltarTile _sw)
                              (Utilities|IsValid _se
                                (:Is%20Valid
                                  (Utilities|ResaltarTile _se))))))))))))))))))