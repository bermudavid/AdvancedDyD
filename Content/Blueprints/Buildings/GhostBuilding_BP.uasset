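; GhostBuilding_BP is a ghost building that shows a placement mesh for a building to be constructed.
; OnSpawn activates it only when inactive, storing the building class, construction proxy class and display mesh, then applying that mesh to GhostBuildingMesh.
; KillGhost clears those references and the active flag so it can be reused, without resetting the mesh component or destroying the actor.
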(event Custom|OnSpawn
  (params (DisplayMesh :type Static%20Mesh%20Object%20Reference) (ConstructionBuildingClass :type Building%20Master%20BP%20Class%20Reference) (ConstructionProxyClass :type Construction%20Proxy%20BP%20Class%20Reference))
  (if (not (Variables|Default|GetIsActive?))
    (Variables|Default|SetBuildingClass ConstructionBuildingClass)
    (Variables|Default|SetConstructionProxy ConstructionProxyClass)
    (Variables|Default|SetDisplayMesh DisplayMesh)
    (Variables|Default|SetIsActive? true)
    (Components|StaticMesh|SetStaticMesh (Variables|Default|GetGhostBuilding_Mesh) (Variables|Default|GetDisplayMesh))))

(event Custom|KillGhost
  (Variables|Default|SetBuildingClass 0)
  (Variables|Default|SetConstructionProxy 0)
  (Variables|Default|SetDisplayMesh 0)
  (Variables|Default|SetIsActive? false))

(fn ConstructionScript)