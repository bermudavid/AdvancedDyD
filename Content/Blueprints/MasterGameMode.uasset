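; Master game mode that spawns a centred grid of Grid actors, sized by GridSize at 100-unit spacing, on BeginPlay.
; CastReference first casts to CameraPawnController but sets its MainGameMode to None, as self is left unconnected.
; FillNeighbours is called last but is empty; its disconnected logic would link eight-way neighbours through EsVecino's offset comparisons.
; Adding spawned cells to the Grid array is also disconnected.
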(event EventBeginPlay
  (bind _gridsize (Variables|Default|GetGridSize))
  (bind _returnvalue (Math|Float|Truncate (.y _gridsize)))
  (bind _returnvalue_2 (Math|Float|Truncate (.x _gridsize)))
  (bind _returnvalue_3 (/ _returnvalue 2))
  (bind _returnvalue_4 (/ _returnvalue_2 2))
  (Utilities|FlowControl|Sequence
    (:then_0
      (Utilities|CastReference))
    (:then_1
      (for _index (range (* _returnvalue_4 -1) _returnvalue_4)
        (for _index_2 (range (* _returnvalue_3 -1) _returnvalue_3)
          (bind _returnvalue_5 (Game|SpawnActorfromClass "/Game/Blueprints/Grid/Grid.Grid_C" (Math|Transform|MakeTransform (Math|Vector|MakeVector (* _index_2 1e+02) (* _index 1e+02) 1.0) "0, 0, 0" "1,1,1.000000") "AdjustIfPossibleButAlwaysSpawn" 0 0)))))
    (:then_2
      (CallFunction|FillNeighbours))))

(fn ConstructionScript)

(fn FillNeighbours)

(fn EsVecino?
  (params (A :type Grid%20Object%20Reference) (B :type Grid%20Object%20Reference))
  (bind _returnvalue (Transformation|GetActorLocation B))
  (bind _returnvalue_2 (Transformation|GetActorLocation A))
  (bind _returnvalue_3 (Math|Vector2D|MakeVector2D (.x _returnvalue) (.y _returnvalue)))
  (bind _returnvalue_4 (Math|Vector2D|MakeVector2D (.x _returnvalue_2) (.y _returnvalue_2)))
  (bind _returnvalue_5 (- _returnvalue_4 _returnvalue_3))
  (bind _returnvalue_6 (/ _returnvalue_5 1e+02))
  (bind _returnvalue_7 (* _returnvalue_6 -1.0))
  (if (== A B)
    (return false "NewEnumerator0")
    (elif (<= (/ (Math|Vector2D|Vector2DLength _returnvalue_5) 1e+02) (Math|Float|Sqrt 2.0))
      (if (Math|Vector|Equal(Vector) _returnvalue_7 "(X=0.000000,Y=1.000000)" 0.0001)
        (LocalVariables|SetE_Neighborgs "NewEnumerator0")
        (elif (Math|Vector|Equal(Vector) _returnvalue_7 "(X=1.000000,Y=1.000000)" 0.0001)
          (LocalVariables|SetE_Neighborgs "NewEnumerator5")
          (elif (Math|Vector|Equal(Vector) _returnvalue_7 "(X=1.000000,Y=0.000000)" 0.0001)
            (LocalVariables|SetE_Neighborgs "NewEnumerator3")
            (elif (Math|Vector|Equal(Vector) _returnvalue_7 "(X=1.000000,Y=-1.000000)" 0.0001)
              (LocalVariables|SetE_Neighborgs "NewEnumerator7")
              (elif (Math|Vector|Equal(Vector) _returnvalue_7 "(X=0.000000,Y=-1.000000)" 0.0001)
                (LocalVariables|SetE_Neighborgs "NewEnumerator1")
                (elif (Math|Vector|Equal(Vector) _returnvalue_7 "(X=-1.000000,Y=-1.000000)" 0.0001)
                  (LocalVariables|SetE_Neighborgs "NewEnumerator6")
                  (elif (Math|Vector|Equal(Vector) _returnvalue_7 "(X=-1.000000,Y=0.000000)" 0.0001)
                    (LocalVariables|SetE_Neighborgs "NewEnumerator2")
                    (elif (Math|Vector|Equal(Vector) _returnvalue_7 "(X=-1.000000,Y=1.000000)" 0.0001)
                      (LocalVariables|SetE_Neighborgs "NewEnumerator4")
                      (else
                        (return false "NewEnumerator0"))))))))))
      (return true (LocalVariables|GetE_Neighborgs))
      (else
        (return false "NewEnumerator0")))))