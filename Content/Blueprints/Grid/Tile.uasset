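; Grid tile actor that highlights while the mouse cursor is over it.
; The construction script adds a single instance at the local origin to its InstancedStaticMesh.
; On cursor over, it creates a new dynamic instance of M_Grid with a green frame color and emission strength, then applies it to the mesh.
; On cursor exit, it restores the plain M_Grid material.
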(event EventBeginPlay)

(event Collision|EventActorBeginOverlap
  (params (OtherActor :type Actor%20Object%20Reference)))

(event EventTick
  (params (DeltaSeconds :type Float%20%28single-precision%29)))

(event MouseInput|EventActorBeginCursorOver
  (bind _instancedstaticmesh (Variables|Default|GetInstancedStaticMesh))
  (bind _returnvalue (Rendering|Material|CreateDynamicMaterialInstance _instancedstaticmesh 0 "/Game/Meshes/Grid/M_Grid.M_Grid" :!class /Script/Engine.PrimitiveComponent))
  (Rendering|Material|SetVectorParameterValue _returnvalue "FrameColor" "(R=0.000000,G=0.575000,B=0.060186,A=1.000000)" :!class /Script/Engine.MaterialInstanceDynamic)
  (Rendering|Material|SetScalarParameterValue _returnvalue "EmisionStrength" 0.5 :!class /Script/Engine.MaterialInstanceDynamic)
  (Rendering|Material|SetMaterial _instancedstaticmesh 0 _returnvalue))

(event MouseInput|EventActorEndCursorOver
  (Rendering|Material|SetMaterial (Variables|Default|GetInstancedStaticMesh) 0 "/Game/Meshes/Grid/M_Grid.M_Grid"))

(fn ConstructionScript
  (Components|InstancedStaticMesh|AddInstance (Variables|Default|GetInstancedStaticMesh) (Math|Transform|MakeTransform "0, 0, 0")))