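; GridBP is an actor that builds a centred grid of tiles at BeginPlay and records each tile's neighbours.
; It adds hierarchical instanced static mesh instances at 100-unit spacing from GridSize, then sets their cull distances.
; AddNeig derives eight neighbour indices from each instance index by offset arithmetic, without bounds checks, and stores them in Vecinos.
; GetNeig linearly searches supplied neighbour data for a tile's list.
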(event EventBeginPlay
  (bind _gridsize (Variables|Default|GetGridSize))
  (bind _returnvalue (/ (.x _gridsize) 2))
  (bind _returnvalue_2 (/ (.y _gridsize) 2))
  (Utilities|FlowControl|Sequence
    (:then_0
      (for _index (range (* _returnvalue -1) _returnvalue)
        (for _index_2 (range (* _returnvalue_2 -1) _returnvalue_2)
          (bind _returnvalue_3 (Components|InstancedStaticMesh|AddInstance (Variables|Default|GetHierarchicalInstancedStaticMesh) (Math|Transform|MakeTransform (Math|Vector|MakeVector (* _index 1e+02) (* _index_2 1e+02) 0.0) "0,0.000000, 0")))
          (bind _vecinosestructure (CallFunction|AddNeig _returnvalue_3))
          (Utilities|Array|Add (Variables|Default|GetVecinos) _vecinosestructure))))
    (:then_1
      (Components|InstancedStaticMesh|SetCullDistances (Variables|Default|GetHierarchicalInstancedStaticMesh) 100 1000))))

(event Collision|EventActorBeginOverlap
  (params (OtherActor :type Actor%20Object%20Reference)))

(event EventTick
  (params (DeltaSeconds :type Float%20%28single-precision%29)))

(fn ConstructionScript)

(fn AddNeig
  (params (casilla :type Integer))
  (bind _gridsize_x (|CollapseGraph_0))
  (bind _returnvalue (+ _gridsize_x 2))
  (bind _returnvalue_2 (+ _gridsize_x 1))
  (return (Utilities|Struct|MakeVecinosEstructure casilla (Utilities|Array|MakeArray (+ casilla 1) (+ casilla -1) (- casilla _returnvalue_2) (- casilla _gridsize_x) (- casilla _returnvalue) (+ casilla _returnvalue_2) (+ casilla _gridsize_x) (+ casilla _returnvalue)))))

(fn GetNeig
  (params (Index :type Integer) (VecinosData :type Array%20of%20Vecinos%20Estructure%20Structures))
  (for _array_element VecinosData
    (if (== (.Casilla (Utilities|Struct|BreakVecinosEstructure _array_element)) Index)
      (return (.vecinos (Utilities|Struct|BreakVecinosEstructure _array_element))))))