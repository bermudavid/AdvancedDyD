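; Player controller for a top-down building game, driving a CameraPawn and handling building placement setup.
; BeginPlay caches the pawn and, for one role, creates the HUD, construction manager and ghost building.
; Input drives zoom-scaled movement with Shift boost, screen-edge scrolling, spring-arm zoom and gated rotation that pauses edge scrolling.
; ConstructBuilding spawns the building class to feed the ghost preview, while Tick repeatedly possesses any valid referenced entity.
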(event EventBeginPlay
  (bind _returnvalue (Math|Transform|MakeTransform "0,0.000000,0.000000"))
  (if (Utilities|Enum|Equal(Enum) (Variables|Default|GetRol) "NewEnumerator0")
    ;[1 1 1] Begin Play
    (Variables|Default|SetbShowMouseCursor true)
    (Utilities|FlowControl|Sequence
      (:then_0
        (Utilities|ReferenceCast :!label _label))
      (:then_1
        (Input|SetInputModeGameandUI self 0 "LockAlways" false)
        (Utilities|CreateHuds)
        (UserInterface|Viewport|AddtoViewport (Variables|References|GetMainHudRef) 0))
      (:then_2
        (bind _returnvalue_2 (Game|SpawnActorfromClass "/Game/Blueprints/Constructions/ConstructionManager_BP.ConstructionManager_BP_C" _returnvalue "AlwaysSpawn" 0 0))
        (Variables|References|SetConstructionManagerRef _returnvalue_2))
      (:then_3
        (bind _returnvalue_3 (Game|SpawnActorfromClass "/Game/Blueprints/Buildings/GhostBuilding_BP.GhostBuilding_BP_C" _returnvalue "AlwaysSpawn" 0 self 0))
        (Variables|References|SetGhostBuildingRef _returnvalue_3)))
    (else
      (Variables|Default|SetbShowMouseCursor true)
      (goto _label))))

(event EventConstructBuilding
  (params (MainBuilding :type Building%20Master%20BP%20Class%20Reference))
  (bind _ghostbuildingref (Variables|References|GetGhostBuildingRef))
  (bind _returnvalue (Game|SpawnActorfromClass MainBuilding (Math|Transform|MakeTransform "0, 0, 0") "Undefined" 0 self 0))
  (bind _asbuilding_master_bp (Utilities|Casting|CastToBuildingMaster_BPClass MainBuilding))
  (Default|KillGhost _ghostbuildingref)
  (Default|OnSpawn _ghostbuildingref (Variables|/Game/Blueprints/Buildings/BuildingMaster_BP.BuildingMaster_BP_C|GetDisplayMesh _returnvalue) _asbuilding_master_bp (Variables|/Game/Blueprints/Buildings/BuildingMaster_BP.BuildingMaster_BP_C|GetConstructionProxy _returnvalue)))

(event EventTick
  (params (DeltaSeconds :type Float%20%28single-precision%29))
  (bind _entitypossesedreference (Variables|References|GetEntityPossesedReference))
  (Utilities|IsValid _entitypossesedreference
    (:Is%20Valid
      (Pawn|Possess _entitypossesedreference))))

(event Input|ActionEvents|InputActionPan
  (params (Key :type Key%20Structure :default "AnyKey"))
  (bind _camerapawnref (Variables|References|GetCameraPawnRef))
  (bind _returnvalue (Transformation|GetActorRotation _camerapawnref))
  (bind (_roll _pitch _yaw) (Math|Rotator|BreakRotator _returnvalue))
  ;[0.05432 1 0.2203] Camera Movement
  ;;[1 1 1] Pan X
  (:Pressed
    (Variables|Default|SetDisableCamNav true)
    (Utilities|FlowControl|Gate true) ; enters at Open
  )
  (:Released
    (Variables|Default|SetDisableCamNav false)
    (Utilities|FlowControl|Gate true) ; enters at Close
  ))

(event Input|ActionEvents|InputActionPan
  (params (Key :type Key%20Structure :default "AnyKey"))
  (bind _camerapawnref (Variables|References|GetCameraPawnRef))
  (bind _returnvalue (Transformation|GetActorRotation _camerapawnref))
  (bind (_roll _pitch _yaw) (Math|Rotator|BreakRotator _returnvalue))
  ;[0.05432 1 0.2203] Camera Movement
  ;;[1 1 1] Pan y
  (:Pressed
    (Variables|Default|SetDisableCamNav true)
    (Utilities|FlowControl|Gate true) ; enters at Open
  )
  (:Released
    (Variables|Default|SetDisableCamNav false)
    (Utilities|FlowControl|Gate true) ; enters at Close
  ))

(event Input|ActionEvents|InputActionPanReset
  (params (Key :type Key%20Structure :default "AnyKey"))
  (bind _camerapawnref (Variables|References|GetCameraPawnRef))
  (bind _returnvalue (Transformation|GetActorRotation _camerapawnref))
  (bind (_roll _pitch _yaw) (Math|Rotator|BreakRotator _returnvalue))
  ;[0.05432 1 0.2203] Camera Movement
  ;;[1 1 1] Pan Reset
  (:Pressed
    (Transformation|SetActorRotation _camerapawnref (Math|Rotator|MakeRotator _roll 0.0 _yaw))))

(event Input|ActionEvents|InputActionZoomIn
  (params (Key :type Key%20Structure :default "AnyKey"))
  (bind (_springarm _targetarmlength) (|SpringArm))
  ;[0.05432 1 0.2203] Camera Movement
  ;;[1 1 1] Zoom
  (:Pressed
    (Variables|/Script/Engine.SpringArmComponent|SetTargetArmLength _springarm (Math|Float|Clamp(Float) (- _targetarmlength (Variables|Default|GetZoomSensitivity)) 5e+02 (Variables|Default|GetMaxArmDistance)))))

(event Input|ActionEvents|InputActionZoomOut
  (params (Key :type Key%20Structure :default "AnyKey"))
  (bind (_springarm _targetarmlength) (|SpringArm))
  ;[0.05432 1 0.2203] Camera Movement
  ;;[1 1 1] Zoom
  (:Pressed
    (Variables|/Script/Engine.SpringArmComponent|SetTargetArmLength _springarm (Math|Float|Clamp(Float) (+ _targetarmlength (Variables|Default|GetZoomSensitivity)) 5e+02 (Variables|Default|GetMaxArmDistance)))))

(event Input|AxisEvents|InputAxisMoveForward
  (params (AxisValue :type Float%20%28single-precision%29))
  ;[0.05432 1 0.2203] Camera Movement
  ;;[1 1 1] Movement X
  (Transformation|SetActorTransform (Variables|References|GetCameraPawnRef) (Utilities|MovementX (CallFunction|MovementSpeedCalculation) (Variables|Default|GetFastMoveMultiplier) AxisValue (Variables|References|GetCameraPawnRef))))

(event Input|AxisEvents|InputAxisMoveRight
  (params (AxisValue :type Float%20%28single-precision%29))
  (bind _movesensitivity (CallFunction|MovementSpeedCalculation))
  (bind _fastmovemultiplier (Variables|Default|GetFastMoveMultiplier))
  (bind _camerapawnref (Variables|References|GetCameraPawnRef))
  (bind _transform (Utilities|MovementY AxisValue _movesensitivity _fastmovemultiplier _camerapawnref))
  (bind (_location _rotation _scale) (Math|Transform|BreakTransform _transform))
  (bind (_x _y) (Math|Vector|BreakVector _location))
  ;[0.05432 1 0.2203] Camera Movement
  ;;[1 1 1] Movement Y
  (Transformation|SetActorTransform (Variables|References|GetCameraPawnRef) (Math|Transform|MakeTransform (Math|Vector|MakeVector _x _y 1e+02) _rotation _scale)))

(event Input|AxisEvents|InputAxisMoveForward2
  (params (AxisValue :type Float%20%28single-precision%29))
  ;[1 1 1] Movement X
  (Transformation|SetActorTransform (Variables|References|GetEntityPossesedReference) (Utilities|MovementX (CallFunction|MovementSpeedCalculation) (Variables|Default|GetFastMoveMultiplier) AxisValue (Variables|References|GetEntityPossesedReference)) false true))

(event Input|MouseEvents|MouseX
  (params (AxisValue :type Float%20%28single-precision%29))
  (bind _camerapawnref (Variables|References|GetCameraPawnRef))
  (bind _returnvalue (Transformation|GetActorRotation _camerapawnref))
  (bind (_roll _pitch _yaw) (Math|Rotator|BreakRotator _returnvalue))
  ;[0.05432 1 0.2203] Camera Movement
  ;;[1 1 1] Pan X
  (Utilities|FlowControl|Gate true
    (:Exit
      (Transformation|SetActorRotation (Variables|References|GetCameraPawnRef) (Math|Rotator|MakeRotator _roll _pitch (+ _yaw (* AxisValue (Variables|Default|GetPanSensitivity))))))))

(event Input|MouseEvents|MouseY
  (params (AxisValue :type Float%20%28single-precision%29))
  (bind _camerapawnref (Variables|References|GetCameraPawnRef))
  (bind _returnvalue (Transformation|GetActorRotation _camerapawnref))
  (bind (_roll _pitch _yaw) (Math|Rotator|BreakRotator _returnvalue))
  ;[0.05432 1 0.2203] Camera Movement
  ;;[1 1 1] Pan y
  (Utilities|FlowControl|Gate true
    (:Exit
      (Transformation|SetActorRotation (Variables|References|GetCameraPawnRef) (Math|Rotator|MakeRotator _roll (Math|Float|Clamp(Float) (+ _pitch (* AxisValue (Variables|Default|GetPanSensitivity))) -15.0 45.0) _yaw)))))

(event Input|MouseEvents|MouseX
  (params (AxisValue :type Float%20%28single-precision%29))
  ;[0.05432 1 0.2203] Camera Movement
  ;;[1 1 1] Automatic movement at the borders of the screen
  (if (not (Variables|Default|GetDisableCamNav))
    (bind (_deltaxspeed _deltayspeed) (Utilities|ScreenEdgeMovement))
    (Transformation|AddActorLocalOffset (Variables|References|GetCameraPawnRef) (Math|Vector|MakeVector _deltayspeed _deltaxspeed 0.0) true false)))

(event Input|MouseEvents|MouseY
  (params (AxisValue :type Float%20%28single-precision%29))
  ;[0.05432 1 0.2203] Camera Movement
  ;;[1 1 1] Automatic movement at the borders of the screen
  (if (not (Variables|Default|GetDisableCamNav))
    (Utilities|ScreenEdgeMovement) ; enters at MouseY
  ))

(event Input|KeyboardEvents|LeftShift
  (params (Key :type Key%20Structure :default "AnyKey"))
  ;[0.05432 1 0.2203] Camera Movement
  ;;[1 1 1] fast move
  (:Pressed
    (Variables|Default|SetFastMoveMultiplier 2.0))
  (:Released
    (Variables|Default|SetFastMoveMultiplier 1.0)))

(fn ConstructionScript)

(fn MovementSpeedCalculation
  (return (Math|Float|Clamp(Float) (/ (Variables|/Script/Engine.SpringArmComponent|GetTargetArmLength (Variables|/Game/Blueprints/CameraPawn.CameraPawn_C|GetSpringArm (Variables|References|GetCameraPawnRef))) 1e+02) 5.0 2e+01)))